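; Electric projectile Blueprint that reacts to actors overlapping its Collision component.
; A BP_TwinStickNPC is destroyed outright, while any other actor except the instigator receives a ProjectileImpactMessage with damage, instigator and a forward vector from zero rotation.
; The projectile does not destroy itself on overlap, and the Niagara activation and target-position nodes are left unconnected.
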(event OnComponentBeginOverlap(Collision)
  (params (OverlappedComponent :type Primitive%20Component%20Object%20Reference) (OtherActor :type Actor%20Object%20Reference) (OtherComp :type Primitive%20Component%20Object%20Reference) (OtherBodyIndex :type Integer) (bFromSweep :type Boolean) (SweepResult :type Hit%20Result%20Structure%20%28by%20ref%29))
  (bind _returnvalue (Game|GetInstigator))
  (if (== OtherActor "/Game/Variant_TwinStick/Blueprints/AI/BP_TwinStickNPC.BP_TwinStickNPC")
    (bind _asbp_twin_stick_npc (Utilities|Casting|CastToBP_TwinStickNPC OtherActor))
    (Actor|DestroyActor _asbp_twin_stick_npc)
    (elif (!= OtherActor _returnvalue)
      (Class|BPITwinstick|ProjectileImpact(Message) OtherActor (Math|Vector|GetForwardVector "0, 0, 0") _returnvalue false 20))))

(fn ConstructionScript)