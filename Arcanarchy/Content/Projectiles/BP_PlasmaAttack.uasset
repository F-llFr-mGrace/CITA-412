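; Plasma attack projectile actor that becomes dangerous after a short delay and destroys itself shortly afterwards.
; BeginPlay and OnSpawn share a timed chain that switches Collision to query-only, waits briefly, then destroys the actor.
; Overlapping actors receive a ProjectileImpactMessage carrying the instigator and damage, with the instigator itself taking half damage when caught in it.
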(event OnComponentBeginOverlap(Collision)
  (params (OverlappedComponent :type Primitive%20Component%20Object%20Reference) (OtherActor :type Actor%20Object%20Reference) (OtherComp :type Primitive%20Component%20Object%20Reference) (OtherBodyIndex :type Integer) (bFromSweep :type Boolean) (SweepResult :type Hit%20Result%20Structure%20%28by%20ref%29))
  (bind _returnvalue (Game|GetInstigator))
  (if (!= OtherActor _returnvalue)
    (Class|BPITwinstick|ProjectileImpact(Message) OtherActor "0, 0, 0" _returnvalue false 30)
    (else
      (Class|BPITwinstick|ProjectileImpact(Message) _returnvalue "0, 0, 0" _returnvalue false 15))))

(event Custom|OnSpawn
  (Utilities|FlowControl|Delay 2.0)
  (Collision|SetCollisionEnabled (Variables|Default|GetCollision) "QueryOnly")
  (Utilities|FlowControl|Delay 1.0)
  (Actor|DestroyActor))

(event EventBeginPlay
  (Utilities|FlowControl|Delay 2.0)
  (Collision|SetCollisionEnabled (Variables|Default|GetCollision) "QueryOnly")
  (Utilities|FlowControl|Delay 1.0)
  (Actor|DestroyActor))

(fn ConstructionScript)