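; BP_Shooter is an actor that fires a single electric projectile shortly after play begins.
; A near-zero, non-looping timer on BeginPlay calls Spawn, which creates the projectile at LightningFirePoint using the owning actor's rotation.
; Spawn then activates the projectile's Niagara effect, assigns a fixed X-axis velocity and disables gravity on its ProjectileMovement.
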(event Custom|Spawn
  (bind _returnvalue (Game|SpawnActorfromClass "/Game/BP_ElectricProjectile.BP_ElectricProjectile_C" (Math|Transform|MakeTransform (Transformation|GetWorldLocation (Variables|Default|GetLightningFirePoint)) (Transformation|GetActorRotation (Components|GetOwner (Variables|Default|GetLightningFirePoint)))) "AlwaysSpawn" "MultiplyWithRoot" 0 0))
  (Components|Activation|SetActive (Variables|/Game/BP_ElectricProjectile.BP_ElectricProjectile_C|GetNiagara _returnvalue) true true)
  (Variables|/Script/Engine.MovementComponent|SetVelocity (Variables|/Game/BP_ElectricProjectile.BP_ElectricProjectile_C|GetProjectileMovement _returnvalue) "2000.000000,0.000000,0.000000")
  (Variables|/Script/Engine.ProjectileMovementComponent|SetProjectileGravityScale (Variables|/Game/BP_ElectricProjectile.BP_ElectricProjectile_C|GetProjectileMovement _returnvalue) 0.0))

(event EventBeginPlay
  (Utilities|Time|SetTimerbyFunctionName 0 "Spawn" 0.001))

(fn ConstructionScript)