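; BP_GI is the Game Instance that handles multiplayer session teardown and connection failures.
; Network and travel error events print the failure type on screen in red, then share a path that destroys the first player's session.
; LeaveSession opens the network test main menu level and destroys the session, then on success destroys the player's BP_TwinStickCharacter.
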(event Custom|LeaveSession
  ;[0.15 0.15 0.15 0.5] Leave Session
  (Game|OpenLevel(byName) "NetworkTest_MainMenu_Level")
  (|DestroySession (Game|GetPlayerController 0)
    (:OnSuccess
      (bind _asbp_twin_stick_character (Utilities|Casting|CastToBP_TwinStickCharacter (Game|GetPlayerCharacter 0)))
      (Actor|DestroyActor _asbp_twin_stick_character))))

(event EventHandleNetworkError
  (params (FailureType :type ENetworkFailure%20Enum :default "NetDriverAlreadyExists") (bIsServer :type Boolean))
  ;[0.15 0.15 0.15 0.5] Handle Network & Travel Errors
  (Development|PrintString (Utilities|String|EnumtoString FailureType) true true "(R=1.000000,G=0.033237,B=0.005062,A=1.000000)" 1e+01)
  (|DestroySession (Game|GetPlayerController 0)))

(event EventHandleTravelError
  (params (FailureType :type ETravelFailure%20Enum :default "NoLevel"))
  ;[0.15 0.15 0.15 0.5] Handle Network & Travel Errors
  (Development|PrintString (Utilities|String|EnumtoString FailureType) true true "(R=1.000000,G=0.003500,B=0.008432,A=1.000000)" 1e+01)
  (|DestroySession (Game|GetPlayerController 0)))